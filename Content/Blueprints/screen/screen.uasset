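; Calculator screen actor that shows typed expressions and results on a TextRender updated every Tick.
; SetAngka and SetOperator build the display and infix token array, re-arming the DoOnce that Equal fires.
; Equal converts infix to postfix by shunting-yard with precedence and parentheses, then evaluates it on a stack, including square and square root.
; CekInfix only prints token-order diagnostics; the result clears after a delay.
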(event `self.ReceiveTick`
  (params (DeltaSeconds :type "Float (single-precision)"))
  (`TextRenderComponent.K2_SetText` (`self.TextRender`) (`self.value`)))

(event `SetAngka`
  (params (Input :type Text))
  (bind _b_layar (`self.b_layar`))
  (bind _operator_temp (`self.operator_Temp`))
  (bind _operator_temp_2 (`self.operator_Temp`))
  (bind _operator_temp_3 (`self.operator_Temp`))
  (bind _operator_temp_4 (`self.operator_Temp`))
  (bind _operator_temp_5 (`self.operator_Temp`))
  (bind _operator_temp_6 (`self.operator_Temp`))
  (bind _operator_temp_7 (`self.operator_Temp`))
  (bind _operator_temp_8 (`self.operator_Temp`))
  (bind _operator_temp_9 (`self.operator_Temp`))
  (bind _operator_temp_10 (`self.operator_Temp`))
  (bind _angka (`self.angka`))
  (bind _angka_2 (`self.angka`))
  (bind _angka_3 (`self.angka`))
  (bind _operator (`self.operator`))
  (bind _operator_2 (`self.operator`))
  (bind _angka_4 (`self.angka`))
  (bind _angka_5 (`self.angka`))
  (bind _angka_6 (`self.angka`))
  (bind _angka_7 (`self.angka`))
  (bind _returnvalue (`KismetTextLibrary.Conv_TextToString` _b_layar))
  (bind _output (`|GetArrayItem` _operator_temp_6 (`KismetArrayLibrary.Array_LastIndex` _operator_temp_6)))
  (bind _output_2 (`|GetArrayItem` _operator_temp_7 (`KismetArrayLibrary.Array_LastIndex` _operator_temp_7)))
  (bind _output_3 (`|GetArrayItem` _operator_temp_10 (`KismetArrayLibrary.Array_LastIndex` _operator_temp_10)))
  (bind _output_4 (`|GetArrayItem` _angka_7 (`KismetArrayLibrary.Array_LastIndex` _angka_7)))
  (`|ExecutionSequence`
    (:`then_0`
      (goto _label :!via `Reset`))
    (:`then_1`
      (set `self.value` (`KismetTextLibrary.Conv_StringToText` (`KismetStringLibrary.Concat_StrStr` (`KismetTextLibrary.Conv_TextToString` (`self.value`)) (`KismetTextLibrary.Conv_TextToString` Input))))
      (set `self.b_layar` (`KismetTextLibrary.Conv_StringToText` (`KismetStringLibrary.Concat_StrStr` (`KismetTextLibrary.Conv_TextToString` (`self.b_layar`)) (`KismetTextLibrary.Conv_TextToString` Input)))))))

(event `SetOperator`
  (params (input1 :type Text))
  (bind _returnvalue (`KismetTextLibrary.Conv_TextToString` input1))
  (bind _b_layar (`self.b_layar`))
  (bind _operator_temp (`self.operator_Temp`))
  (bind _operator_temp_2 (`self.operator_Temp`))
  (bind _operator_temp_3 (`self.operator_Temp`))
  (bind _operator_temp_4 (`self.operator_Temp`))
  (bind _operator_temp_5 (`self.operator_Temp`))
  (bind _operator_temp_6 (`self.operator_Temp`))
  (bind _operator_temp_7 (`self.operator_Temp`))
  (bind _operator_temp_8 (`self.operator_Temp`))
  (bind _operator_temp_9 (`self.operator_Temp`))
  (bind _operator_temp_10 (`self.operator_Temp`))
  (bind _angka (`self.angka`))
  (bind _angka_2 (`self.angka`))
  (bind _angka_3 (`self.angka`))
  (bind _operator (`self.operator`))
  (bind _operator_2 (`self.operator`))
  (bind _angka_4 (`self.angka`))
  (bind _angka_5 (`self.angka`))
  (bind _angka_6 (`self.angka`))
  (bind _angka_7 (`self.angka`))
  (bind _returnvalue_2 (`KismetTextLibrary.Conv_TextToString` _b_layar))
  (bind _returnvalue_3 (`KismetTextLibrary.Conv_TextToString` (`self.b_layar`)))
  (bind _output (`|GetArrayItem` _operator_temp_6 (`KismetArrayLibrary.Array_LastIndex` _operator_temp_6)))
  (bind _output_2 (`|GetArrayItem` _operator_temp_7 (`KismetArrayLibrary.Array_LastIndex` _operator_temp_7)))
  (bind _output_3 (`|GetArrayItem` _operator_temp_10 (`KismetArrayLibrary.Array_LastIndex` _operator_temp_10)))
  (bind _output_4 (`|GetArrayItem` _angka_7 (`KismetArrayLibrary.Array_LastIndex` _angka_7)))
  (`|ExecutionSequence`
    (:`then_0`
      (goto _label :!via `Reset`))
    (:`then_1`
      (set `self.value` (`KismetTextLibrary.Conv_StringToText` (`KismetStringLibrary.Concat_StrStr` (`KismetTextLibrary.Conv_TextToString` (`self.value`)) (`KismetTextLibrary.Conv_TextToString` input1))))
      (`KismetSystemLibrary.PrintString` (`KismetStringLibrary.Concat_StrStr` "mengisi infix 1 : " _returnvalue_3))
      (`KismetArrayLibrary.Array_Add` (`self.infix`) _returnvalue_3)
      (`KismetSystemLibrary.PrintString` (`KismetStringLibrary.Concat_StrStr` "mengisi infix 2 : " _returnvalue))
      (`KismetArrayLibrary.Array_Add` (`self.infix`) _returnvalue)
      (set `self.b_layar` ""))))

(event `Equal`
  (bind _b_layar (`self.b_layar`))
  (bind _operator_temp (`self.operator_Temp`))
  (bind _operator_temp_2 (`self.operator_Temp`))
  (bind _operator_temp_3 (`self.operator_Temp`))
  (bind _operator_temp_4 (`self.operator_Temp`))
  (bind _operator_temp_5 (`self.operator_Temp`))
  (bind _operator_temp_6 (`self.operator_Temp`))
  (bind _operator_temp_7 (`self.operator_Temp`))
  (bind _operator_temp_8 (`self.operator_Temp`))
  (bind _operator_temp_9 (`self.operator_Temp`))
  (bind _operator_temp_10 (`self.operator_Temp`))
  (bind _angka (`self.angka`))
  (bind _angka_2 (`self.angka`))
  (bind _angka_3 (`self.angka`))
  (bind _operator (`self.operator`))
  (bind _operator_2 (`self.operator`))
  (bind _angka_4 (`self.angka`))
  (bind _angka_5 (`self.angka`))
  (bind _angka_6 (`self.angka`))
  (bind _angka_7 (`self.angka`))
  (bind _returnvalue (`KismetTextLibrary.Conv_TextToString` _b_layar))
  (bind _output (`|GetArrayItem` _operator_temp_6 (`KismetArrayLibrary.Array_LastIndex` _operator_temp_6)))
  (bind _output_2 (`|GetArrayItem` _operator_temp_7 (`KismetArrayLibrary.Array_LastIndex` _operator_temp_7)))
  (bind _output_3 (`|GetArrayItem` _operator_temp_10 (`KismetArrayLibrary.Array_LastIndex` _operator_temp_10)))
  (bind _output_4 (`|GetArrayItem` _angka_7 (`KismetArrayLibrary.Array_LastIndex` _angka_7)))
  (`/Engine/EditorBlueprintResources/StandardMacros.DoOnce` false :!label _label
    (:`Completed`
      (set `self.Kosongg` "")
      (if (not (`KismetTextLibrary.EqualEqual_TextText` _b_layar (`self.Kosongg`)))
        (`KismetArrayLibrary.Array_Add` (`self.infix`) _returnvalue)
        (`KismetSystemLibrary.PrintString` (`KismetStringLibrary.Concat_StrStr` "mengisi infix 2 : " _returnvalue)))
      (`self.cek_infix` (`self.infix`))
      (for _array_element (`self.infix`)
        (`KismetSystemLibrary.PrintString` (`KismetStringLibrary.Concat_StrStr` "isi infix sekarang : " _array_element))
        (if (`KismetStringLibrary.EqualEqual_StrStr` _array_element "-")
          (if (== _array_element "(") :!label _label_2
            (`KismetArrayLibrary.Array_Add` (`self.operator_Temp`) _array_element)
            (elif (== _array_element ")")
              (`KismetSystemLibrary.PrintString` "Hello")
              (while (and (not (`KismetArrayLibrary.Array_IsEmpty` (`self.operator_Temp`))) (not (== (`|GetArrayItem` _operator_temp_4 (`KismetArrayLibrary.Array_LastIndex` _operator_temp_4)) "(")))
                (`KismetSystemLibrary.PrintString` (`KismetStringLibrary.Concat_StrStr` "mengisi postfix 2 : " _output_2))
                (`KismetArrayLibrary.Array_Add` (`self.postfix`) _output_2)
                (`KismetArrayLibrary.Array_Remove` _operator_temp_8 (`KismetArrayLibrary.Array_LastIndex` _operator_temp_8)))
              (if (and (`KismetArrayLibrary.Array_IsNotEmpty` (`self.operator_Temp`)) (== (`|GetArrayItem` _operator_temp (`KismetArrayLibrary.Array_LastIndex` _operator_temp)) "("))
                (`KismetArrayLibrary.Array_Remove` _operator_temp_2 (`KismetArrayLibrary.Array_LastIndex` _operator_temp_2)))
              (else
                (`KismetSystemLibrary.PrintString` "hi")
                (while (and (not (`KismetArrayLibrary.Array_IsEmpty` (`self.operator_Temp`))) (<= (`self.Precedence` _array_element) (`self.Precedence` (`|GetArrayItem` _operator_temp_3 (`KismetArrayLibrary.Array_LastIndex` _operator_temp_3)))))
                  (`KismetSystemLibrary.PrintString` "hi 1")
                  (`KismetSystemLibrary.PrintString` (`KismetStringLibrary.Concat_StrStr` "mengisi postfix 3 : " _output))
                  (`KismetArrayLibrary.Array_Add` (`self.postfix`) _output)
                  (`KismetSystemLibrary.PrintString` "hi 2")
                  (`KismetArrayLibrary.Array_Remove` _operator_temp_5 (`KismetArrayLibrary.Array_LastIndex` _operator_temp_5)))
                (`KismetSystemLibrary.PrintString` "hi 3")
                (`KismetArrayLibrary.Array_Add` (`self.operator_Temp`) _array_element))))
          (elif (`KismetStringLibrary.EqualEqual_StrStr` _array_element "+")
            (goto _label_2)
            (elif (`KismetStringLibrary.IsNumeric` _array_element)
              (`KismetArrayLibrary.Array_Add` (`self.postfix`) _array_element)
              (`KismetSystemLibrary.PrintString` (`KismetStringLibrary.Concat_StrStr` "mengisi postfix 1 : " _array_element))
              (else
                (goto _label_2))))))
      (while (`KismetArrayLibrary.Array_IsNotEmpty` (`self.operator_Temp`))
        (`KismetSystemLibrary.PrintString` (`KismetStringLibrary.Concat_StrStr` "mengisi postfix : " _output_3))
        (`KismetArrayLibrary.Array_Add` (`self.postfix`) _output_3)
        (`KismetArrayLibrary.Array_Remove` _operator_temp_9 (`KismetArrayLibrary.Array_LastIndex` _operator_temp_9)))
      ;[1 1 1] print Postfix
      (for (_array_element_2 _array_index) (`self.postfix`)
        (if (== _array_index 0)
          (set `self.hasil` _array_element_2)
          (else
            (set `self.hasil` (`KismetStringLibrary.Concat_StrStr` (`self.hasil`) _array_element_2))
            (set `self.pertama` _array_element_2))))
      (`KismetSystemLibrary.PrintString` (`KismetStringLibrary.Concat_StrStr` "ini print terakhir : " (`self.hasil`) "."))
      ;[1 1 1] membuat hasil
      (for _array_element_3 (`self.postfix`)
        (`KismetSystemLibrary.PrintString` (`KismetStringLibrary.Concat_StrStr` "masuk loop : " _array_element_3))
        (if (`KismetStringLibrary.EqualEqual_StrStr` _array_element_3 "-")
          (`KismetSystemLibrary.PrintString` "masuk 1")
          (`KismetArrayLibrary.Array_Add` (`self.operator`) _array_element_3 :!label _label_3)
          (if (`KismetStringLibrary.EqualEqual_StrStr` _array_element_3 "^2")
            (bind _hasil (`self.applyOperator_2` (`|GetArrayItem` _angka_5 (`KismetArrayLibrary.Array_LastIndex` _angka_5)) _array_element_3 :!label _label_4))
            (for _array_element_4 (`self.angka`)
              (`KismetSystemLibrary.PrintString` (`KismetStringLibrary.Concat_StrStr` " isi angka sebelum remove : " _array_element_4)))
            (`KismetArrayLibrary.Array_Remove` _angka_3 (`KismetArrayLibrary.Array_LastIndex` _angka_3))
            (`KismetSystemLibrary.PrintString` (`KismetStringLibrary.Concat_StrStr` "mengisi angka hasil :" _hasil))
            (`KismetArrayLibrary.Array_Add` (`self.angka`) _hasil)
            (for _array_element_5 (`self.angka`)
              (`KismetSystemLibrary.PrintString` (`KismetStringLibrary.Concat_StrStr` " isi angka setelah add : " _array_element_5)))
            (`KismetArrayLibrary.Array_Remove` _operator (`KismetArrayLibrary.Array_LastIndex` _operator))
            (else
              (`KismetSystemLibrary.PrintString` "ini false")
              (if (`KismetStringLibrary.EqualEqual_StrStr` _array_element_3 "^0.5")
                (`KismetSystemLibrary.PrintString` "trueeee")
                (goto _label_4)
                (else
                  (bind _hasil_2 (`self.applyOperator` (`|GetArrayItem` _angka_4 (- (`KismetArrayLibrary.Array_LastIndex` _angka_4) 1)) (`|GetArrayItem` _angka_6 (`KismetArrayLibrary.Array_LastIndex` _angka_6)) _array_element_3))
                  (`KismetArrayLibrary.Array_Remove` _angka_2 (`KismetArrayLibrary.Array_LastIndex` _angka_2))
                  (`KismetArrayLibrary.Array_Remove` _angka (`KismetArrayLibrary.Array_LastIndex` _angka))
                  (`KismetArrayLibrary.Array_Add` (`self.angka`) _hasil_2)
                  (`KismetArrayLibrary.Array_Remove` _operator_2 (`KismetArrayLibrary.Array_LastIndex` _operator_2))))))
          (elif (`KismetStringLibrary.EqualEqual_StrStr` _array_element_3 "+")
            (`KismetSystemLibrary.PrintString` "masuk 2")
            (goto _label_3)
            (elif (`KismetStringLibrary.IsNumeric` _array_element_3)
              (`KismetSystemLibrary.PrintString` "ini masuk angka")
              (`KismetArrayLibrary.Array_Add` (`self.angka`) _array_element_3)
              (else
                (`KismetSystemLibrary.PrintString` "masuk 3")
                (goto _label_3))))))
      ;[1 1 1] menampilkan hasil
      (`KismetSystemLibrary.PrintString` (`KismetStringLibrary.Concat_StrStr` "Hasil akhir :" _output_4))
      (set `self.value` (`KismetTextLibrary.Conv_StringToText` _output_4))
      (`KismetSystemLibrary.Delay` 5.0)
      ;[1 1 1] reset
      (`KismetArrayLibrary.Array_Clear` (`self.angka`))
      (`KismetArrayLibrary.Array_Clear` (`self.postfix`))
      (`KismetArrayLibrary.Array_Clear` (`self.operator_Temp`))
      (`KismetArrayLibrary.Array_Clear` (`self.infix`))
      (`KismetArrayLibrary.Array_Clear` (`self.operator`))
      (set `self.angka_Simpanan` "")
      (set `self.b_layar` "")
      (set `self.cek_sebelum` "")
      (set `self.cek_sekarang` "")
      (set `self.pertama` "")
      (set `self.sekarang` "")
      (set `self.hasil` "")
      (set `self.value` ""))))

(event `InfixToPostif`
  (for _ (`self.infix`)
    _))

(fn `applyOperator`
  (params (atas :type String) (bawah :type String) (Operator :type String))
  (returns (hasil :type String))
  (if (`KismetStringLibrary.EqualEqual_StrStr` Operator "+")
    (return (`KismetStringLibrary.Conv_DoubleToString` (+ (`KismetStringLibrary.Conv_StringToDouble` atas) (`KismetStringLibrary.Conv_StringToDouble` bawah))))
    (elif (`KismetStringLibrary.EqualEqual_StrStr` Operator "-")
      (return (`KismetStringLibrary.Conv_DoubleToString` (- (`KismetStringLibrary.Conv_StringToDouble` atas) (`KismetStringLibrary.Conv_StringToDouble` bawah))))
      (elif (`KismetStringLibrary.EqualEqual_StrStr` Operator "X")
        (return (`KismetStringLibrary.Conv_DoubleToString` (* (`KismetStringLibrary.Conv_StringToDouble` atas) (`KismetStringLibrary.Conv_StringToDouble` bawah))))
        (elif (`KismetStringLibrary.EqualEqual_StrStr` Operator "/")
          (return (`KismetStringLibrary.Conv_DoubleToString` (/ (`KismetStringLibrary.Conv_StringToDouble` atas) (`KismetStringLibrary.Conv_StringToDouble` bawah)))))))))

(fn `applyOperator_2`
  (params (atas :type String) (Operator :type String))
  (returns (hasil :type String))
  (if (`KismetStringLibrary.EqualEqual_StrStr` Operator "^2")
    (return (`KismetStringLibrary.Conv_DoubleToString` (`KismetMathLibrary.Square` (`KismetStringLibrary.Conv_StringToDouble` atas))))
    (elif (`KismetStringLibrary.EqualEqual_StrStr` Operator "^0.5")
      (return (`KismetStringLibrary.Conv_DoubleToString` (`KismetMathLibrary.Sqrt` (`KismetStringLibrary.Conv_StringToDouble` atas)))))))

(fn `cek_infix`
  (params (infix :type "Array of String"))
  (for (_array_element _array_index) infix
    (if (== _array_index 0)
      (set `self.cek_sebelum` _array_element)
      (else
        (set `self.cek_sekarang` _array_element)
        (if (and (== (`KismetStringLibrary.IsNumeric` (`self.cek_sekarang`)) true) (== (`KismetStringLibrary.IsNumeric` (`self.cek_sebelum`)) true))
          (`KismetSystemLibrary.PrintString` "ANGKA LALU ANGLA LAGI")
          (break)
          (elif (and (== (`KismetStringLibrary.IsNumeric` (`self.cek_sekarang`)) false) (== (`KismetStringLibrary.IsNumeric` (`self.cek_sebelum`)) false))
            (`KismetSystemLibrary.PrintString` "SETELAH OPERATOR GABOLEH OPERATOR LAGI")
            (break)
            (elif (or (and (== (`KismetStringLibrary.IsNumeric` (`self.cek_sekarang`)) true) (== (`KismetStringLibrary.IsNumeric` (`self.cek_sebelum`)) false)) (and (== (`KismetStringLibrary.IsNumeric` (`self.cek_sekarang`)) false) (== (`KismetStringLibrary.IsNumeric` (`self.cek_sebelum`)) true)))
              (`KismetSystemLibrary.PrintString` "BENERR KERENNN")
              (set `self.cek_sebelum` _array_element))))))))

(fn `Precedence`
  (params (operator :type String))
  (returns (return :type Integer))
  (if (`KismetStringLibrary.EqualEqual_StrStr` operator "+")
    (return 1)
    (elif (`KismetStringLibrary.EqualEqual_StrStr` operator "-")
      (return 1)
      (elif (`KismetStringLibrary.EqualEqual_StrStr` operator "X")
        (return 2)
        (elif (`KismetStringLibrary.EqualEqual_StrStr` operator "/")
          (return 2)
          (elif (`KismetStringLibrary.EqualEqual_StrStr` operator "^2")
            (return 2)
            (elif (`KismetStringLibrary.EqualEqual_StrStr` operator "^0.5")
              (return 2)
              (else
                (return 0)))))))))

(fn `UserConstructionScript`)