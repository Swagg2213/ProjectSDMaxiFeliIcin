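; Floor button (tombol) that types its Value onto the Screen actor when a BP_ThirdPersonCharacter steps on it.
; The construction script shows Value on a TextRender, and BeginPlay finds the Screen actor by class.
; Box overlap appends Value to the screen text once and lowers the button through the Plate timeline.
; Leaving reverses a separate timeline, Timeline, to drive the button height, then resets the DoOnce when it finishes.
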(event `self.ReceiveBeginPlay`
  (bind _returnvalue (`GameplayStatics.GetActorOfClass` "/Game/Blueprints/screen/screen.screen_C"))
  (set `self.Screen` _returnvalue))

(event `self.Box.OnComponentBeginOverlap`
  (params (OverlappedComponent :type "PrimitiveComponent Object Reference") (OtherActor :type "Actor Object Reference") (OtherComp :type "PrimitiveComponent Object Reference") (OtherBodyIndex :type Integer) (bFromSweep :type Boolean) (SweepResult :type "HitResult Structure (by ref)"))
  (bind _screen (`self.Screen`))
  (cast `/Game/ThirdPerson/Blueprints/BP_ThirdPersonCharacter` OtherActor)
  (`/Engine/EditorBlueprintResources/StandardMacros.DoOnce` false :!label _label
    (:`Completed`
      (set `/Game/Blueprints/screen/screen.value` (`KismetTextLibrary.Conv_StringToText` (`KismetStringLibrary.Concat_StrStr` (`KismetTextLibrary.Conv_TextToString` (`/Game/Blueprints/screen/screen.value` _screen)) (`KismetTextLibrary.Conv_TextToString` (`self.Value`)))) _screen)
      (bind (_direction _height) (`Timeline|plate`)
        (:`Update`
          (`SceneComponent.K2_SetRelativeLocation` (`self.tombol`) (`KismetMathLibrary.MakeVector` 100.0 120.0 (`KismetMathLibrary.Lerp` 5.0 -5.0 _height)) false false))))))

(event `self.Box.OnComponentEndOverlap`
  (params (OverlappedComponent :type "PrimitiveComponent Object Reference") (OtherActor :type "Actor Object Reference") (OtherComp :type "PrimitiveComponent Object Reference") (OtherBodyIndex :type Integer))
  (cast `/Game/ThirdPerson/Blueprints/BP_ThirdPersonCharacter` OtherActor)
  (bind (_direction _height) (`Timeline|Timeline` :!via `Reverse`)
    (:`Update`
      (`SceneComponent.K2_SetRelativeLocation` (`self.tombol`) (`KismetMathLibrary.MakeVector` 100.0 120.0 (`KismetMathLibrary.Lerp` 5.0 -5.0 _height)) false false))
    (:`Finished`
      (goto _label :!via `Reset`))))

(fn `UserConstructionScript`
  (`TextRenderComponent.K2_SetText` (`self.TextRender`) (`self.Value`)))