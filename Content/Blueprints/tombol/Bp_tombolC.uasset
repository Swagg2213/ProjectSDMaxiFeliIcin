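; Floor-style clear (C) button that resets a calculator-like Screen when the third-person character steps into its Box.
; Overlap passes a DoOnce, empties the screen's Value, and plays a timeline that lowers the Tombol component.
; Each timeline update also blanks BLayar and removes Infix entries by index while looping.
; End overlap reverses a second timeline to move the button back, re-arming the DoOnce when finished.
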(event `self.Box.OnComponentBeginOverlap`
  (params (OverlappedComponent :type "PrimitiveComponent Object Reference") (OtherActor :type "Actor Object Reference") (OtherComp :type "PrimitiveComponent Object Reference") (OtherBodyIndex :type Integer) (bFromSweep :type Boolean) (SweepResult :type "HitResult Structure (by ref)"))
  (bind _screen (`self.Screen`))
  (bind _infix (`/Game/Blueprints/screen/screen.infix` _screen))
  (cast `/Game/ThirdPerson/Blueprints/BP_ThirdPersonCharacter` OtherActor)
  (`/Engine/EditorBlueprintResources/StandardMacros.DoOnce` false :!label _label
    (:`Completed`
      (set `/Game/Blueprints/screen/screen.value` "" (`self.Screen`))
      (bind (_direction _height) (`Timeline|Timeline_0_0`)
        (:`Update`
          (`SceneComponent.K2_SetRelativeLocation` (`self.tombol`) (`KismetMathLibrary.MakeVector` 100.0 120.0 (`KismetMathLibrary.Lerp` 5.0 -5.0 _height)) false false)
          (set `/Game/Blueprints/screen/screen.b_layar` "" _screen)
          (for (_ _array_index) _infix
            (`KismetArrayLibrary.Array_Remove` _infix _array_index)))))))

(event `self.Box.OnComponentEndOverlap`
  (params (OverlappedComponent :type "PrimitiveComponent Object Reference") (OtherActor :type "Actor Object Reference") (OtherComp :type "PrimitiveComponent Object Reference") (OtherBodyIndex :type Integer))
  (cast `/Game/ThirdPerson/Blueprints/BP_ThirdPersonCharacter` OtherActor)
  (bind (_direction _height) (`Timeline|Timeline_1` :!via `Reverse`)
    (:`Update`
      (`SceneComponent.K2_SetRelativeLocation` (`self.tombol`) (`KismetMathLibrary.MakeVector` 100.0 120.0 (`KismetMathLibrary.Lerp` 5.0 -5.0 _height)) false false))
    (:`Finished`
      (goto _label :!via `Reset`))))

(fn `UserConstructionScript`
  (`parent.UserConstructionScript`))